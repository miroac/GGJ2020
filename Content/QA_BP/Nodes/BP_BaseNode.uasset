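; Base circuit node with input and output states that the player links with lasers, with empty TurnOn and DeactivateNode events.
; Selecting an output spawns a BP_Laser grabbed by the player's gun.
; While unlinked, Tick line-traces to the player and releases the connection if blocked.
; ActivateNode pulses the laser and delays TurnOn by distance to LinkedCircuit, while PowerDown clears laser and connection.
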(event `TurnOn`)

(event `DeactivateNode`)

(event `ActivateNode`
  (bind _output_get (set `self.SignalSpeed` (/ (`self.GetDistanceTo` (`self.LinkedCircuit`)) 1000.0)))
  (`/Game/QAGGJ/Effects/Laser/BP_Laser.TriggerPower` (`self.Laser`) _output_get)
  (`KismetSystemLibrary.PrintString` (`KismetStringLibrary.Conv_DoubleToString` _output_get))
  (`KismetSystemLibrary.Delay` _output_get)
  (`KismetSystemLibrary.PrintString` "Do Something")
  (`self.TurnOn`))

(event `self.ReceiveBeginPlay`
  (set `self.CurrentActivatedNode` "NewEnumerator2")
  (set `self.ActiveOutputNode` "NewEnumerator3")
  (set `self.ActiveInputNode` "NewEnumerator3")
  (bind _asfirst_person_character (cast `/Game/FirstPersonBP/Blueprints/FirstPersonCharacter` (`GameplayStatics.GetPlayerCharacter` 0)))
  (set `self.PlayerCharacterReference` _asfirst_person_character))

(event `self.ReceiveTick`
  (params (DeltaSeconds :type "Float (single-precision)"))
  (if (`|EnumEquality` (`self.ActiveOutputNode`) "NewEnumerator2")
    (`/Engine/EditorBlueprintResources/StandardMacros.IsValid` (`self.LinkedCircuit`)
      (:`Is Not Valid`
        (if (not (`|EnumEquality` (`self.CurrentActivatedNode`) "NewEnumerator0"))
          (bind _outhit (`KismetSystemLibrary.LineTraceSingle` :`Start` (`SceneComponent.K2_GetComponentLocation` (`self.OutputNode`)) :`End` (`SceneComponent.K2_GetComponentLocation` (`Character.Mesh` (`self.PlayerCharacterReference`))) :`TraceChannel` "TraceTypeQuery1" :`DrawDebugType` "Persistent"))
          (bind (_bblockinghit _binitialoverlap _time _distance _location _impactpoint _normal _impactnormal _physmat _hitactor _hitcomponent) (`GameplayStatics.BreakHitResult` _outhit))
          (if _bblockinghit
            (`KismetSystemLibrary.PrintString` (`KismetSystemLibrary.GetDisplayName` _hitcomponent))
            (`/Game/FirstPersonBP/Blueprints/FirstPersonCharacter.ReleaseConnection` (`self.PlayerCharacterReference`))
            (`/Game/QAGGJ/Effects/Laser/BP_Laser.DeactivateLaser` (`self.Laser`))))))))

(event `SetActiveNode`
  (params (HitNode :type String))
  (if (`KismetStringLibrary.Contains` HitNode "output")
    (set `self.ActiveOutputNode` "NewEnumerator2")
    (set `self.CurrentActivatedNode` "NewEnumerator1")
    (bind _returnvalue (`|SpawnActorFromClass` "/Game/QAGGJ/Effects/Laser/BP_Laser.BP_Laser_C" (`KismetMathLibrary.MakeTransform` (`SceneComponent.GetSocketLocation` (`self.OutputNode`) "LaserSocket")) "Undefined" "OverrideRootScale" null null))
    (bind _output_get (set `self.Laser` _returnvalue))
    (`/Game/QAGGJ/Effects/Laser/BP_Laser.ActivateLaser` _returnvalue)
    (`/Game/QAGGJ/Effects/Laser/BP_Laser.ActivateLaser` _output_get)
    (`/Game/QAGGJ/Effects/Laser/BP_Laser.LaserGrabbed` _returnvalue (`/Game/FirstPersonBP/Blueprints/FirstPersonCharacter.FP_Gun` (`self.PlayerCharacterReference`)))
    (`/Game/QAGGJ/Effects/Laser/BP_Laser.LaserGrabbed` _output_get (`/Game/FirstPersonBP/Blueprints/FirstPersonCharacter.FP_Gun` (`self.PlayerCharacterReference`)))
    (else
      (set `self.ActiveInputNode` "NewEnumerator2")
      (set `self.CurrentActivatedNode` "NewEnumerator0"))))

(event `PowerDown`
  (bind _laser (`self.Laser`))
  (`self.DeactivateNode`)
  (set `self.ActiveInputNode` "NewEnumerator2")
  (set `self.ActiveOutputNode` "NewEnumerator2")
  (set `self.CurrentActivatedNode` "NewEnumerator0")
  (`/Engine/EditorBlueprintResources/StandardMacros.IsValid` _laser
    (:`Is Valid`
      (`/Game/QAGGJ/Effects/Laser/BP_Laser.DeactivateLaser` _laser)
      (set `self.Laser` null))
    (:`Is Not Valid`
      _))
  (`/Game/FirstPersonBP/Blueprints/FirstPersonCharacter.ReleaseConnection` (`self.PlayerCharacterReference`))
  (set `self.bPoweredOn?` false))

(fn `UserConstructionScript`)