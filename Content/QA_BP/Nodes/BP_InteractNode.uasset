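; BP_InteractNode is a circuit node Blueprint that switches a referenced world actor on and off.
; ActivateNode defers to the parent, while Turnon checks PoweredOn before calling ActivateItem on ActorToInteractWith and passing activation to a valid LinkedCircuit.
; DeactivateNode calls DeactivateItem on that actor without calling the parent or propagating to the linked circuit.
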(event `self.ActivateNode`
  (`parent.ActivateNode`))

(event `self.TurnOn`
  (bind _linkedcircuit (`self.LinkedCircuit`))
  (if (`self.bPoweredOn?`)
    (`/Game/QA_BP/MISC/BP_BaseMovingObject.ActivateItem` (`self.ActorToInteractWith`))
    (`/Engine/EditorBlueprintResources/StandardMacros.IsValid` _linkedcircuit
      (:`Is Valid`
        (`self.ActivateNode` _linkedcircuit)))))

(event `self.DeactivateNode`
  (`/Game/QA_BP/MISC/BP_BaseMovingObject.DeactivateItem` (`self.ActorToInteractWith`)))

(fn `UserConstructionScript`
  (`parent.UserConstructionScript`))