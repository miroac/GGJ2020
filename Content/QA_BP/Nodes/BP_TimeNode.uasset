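; BP_TimeNode is a timer node in a circuit that passes activation on to a linked circuit after a delay.
; ActivateNode waits TimerDelay, derives SignalSpeed from the distance to LinkedCircuit and triggers the Laser with it.
; It then shares the Turnon path, which waits that travel time and activates LinkedCircuit if PoweredOn is set.
; Debug prints remain along the chain.
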(event `self.ReceiveBeginPlay`
  (`parent.ReceiveBeginPlay`))

(event `self.ReceiveTick`
  (params (DeltaSeconds :type "Float (single-precision)"))
  (`parent.ReceiveTick` DeltaSeconds))

(event `self.TurnOn`
  (`KismetSystemLibrary.Delay` (stale `self.ActivateNode` _output_get) :!label _label)
  (`KismetSystemLibrary.PrintString` "Do Something")
  (if (`self.bPoweredOn?`)
    (`self.ActivateNode` (`self.LinkedCircuit`))))

(event `self.ActivateNode`
  (`KismetSystemLibrary.Delay` (`self.TimerDelay`))
  (bind _output_get (set `self.SignalSpeed` (/ (`self.GetDistanceTo` (`self.LinkedCircuit`)) 1000.0)))
  (`/Game/QAGGJ/Effects/Laser/BP_Laser.TriggerPower` (`self.Laser`) _output_get)
  (`KismetSystemLibrary.PrintString` (`KismetStringLibrary.Conv_DoubleToString` _output_get))
  (goto _label))

(fn `UserConstructionScript`
  (`parent.UserConstructionScript`))