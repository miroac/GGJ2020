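; BP_StartNode is the starting node of a linked node circuit, built on a parent node Blueprint.
; Its Turnon event activates the LinkedCircuit if that reference is valid, while ActivateNode, BeginPlay and Tick only call the parent.
; The construction script removes the inherited InputNode component after running the parent's, leaving the node without an input.
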(event `self.ActivateNode`
  (`parent.ActivateNode`))

(event `self.TurnOn`
  (bind _linkedcircuit (`self.LinkedCircuit`))
  (`/Engine/EditorBlueprintResources/StandardMacros.IsValid` _linkedcircuit
    (:`Is Valid`
      (`self.ActivateNode` _linkedcircuit))))

(event `self.ReceiveBeginPlay`
  (`parent.ReceiveBeginPlay`))

(event `self.ReceiveTick`
  (params (DeltaSeconds :type "Float (single-precision)"))
  (`parent.ReceiveTick` DeltaSeconds))

(fn `UserConstructionScript`
  (`parent.UserConstructionScript`)
  (`ActorComponent.K2_DestroyComponent` (`self.InputNode`)))