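; BP_CompileButton is an activatable button that toggles a node-based compiler on and off.
; ActivateObject flips the running state, and a Timeline lerps the button mesh down when starting and back up when stopping.
; Turning on activates the referenced StartNodeToRun, printing a warning if it is missing.
; Turning off calls PowerDown on every BP_BaseNode actor in the level.
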(event `self.ReceiveBeginPlay`
  (bind _relativelocation (`SceneComponent.RelativeLocation` (`self.Button`)))
  ;[1 1 1] Begin Play
  (`parent.ReceiveBeginPlay`)
  (set `self.Start` _relativelocation)
  (set `self.End` (- _relativelocation (0.0 0.0 10.0))))

(event `TurnOffCompiler`
  ;[1 1 1] Animate button + activate nodes
  (set `self.bIsCompilerRunning?` false)
  (`KismetSystemLibrary.PrintString` "off")
  (`|ExecutionSequence`
    (:`then_0`
      (bind (_direction _newtrack_0) (`Timeline|Timeline` :!via `Reverse` :!label _label)
        (:`Update`
          (`SceneComponent.K2_SetRelativeLocation` (`self.Button`) (`KismetMathLibrary.VLerp` (`self.Start`) (`self.End`) _newtrack_0) false false))))
    (:`then_1`
      (bind _outactors (`GameplayStatics.GetAllActorsOfClass` "/Game/QA_BP/Nodes/BP_BaseNode.BP_BaseNode_C"))
      (for _array_element _outactors
        (`/Game/QA_BP/Nodes/BP_BaseNode.PowerDown` _array_element)))))

(event `self.ActivateObject`
  (params (ComponentHit :type "PrimitiveComponent Object Reference"))
  ;[1 1 1] Animate button + activate nodes
  (if (`self.bIsCompilerRunning?`)
    (`self.TurnOffCompiler`)
    (else
      (`self.TurnOnCompiler`))))

(event `TurnOnCompiler`
  (bind _startnodetorun (`self.StartNodeToRun`))
  ;[1 1 1] Animate button + activate nodes
  (`KismetSystemLibrary.PrintString` "On")
  (set `self.bIsCompilerRunning?` true)
  (`|ExecutionSequence`
    (:`then_0`
      (goto _label))
    (:`then_1`
      (`/Engine/EditorBlueprintResources/StandardMacros.IsValid` _startnodetorun
        (:`Is Valid`
          (`/Game/QA_BP/Nodes/BP_BaseNode.ActivateNode` _startnodetorun))
        (:`Is Not Valid`
          (`KismetSystemLibrary.PrintString` "COMPILER NODE DOES NOT HAVE A START NODE REFERENCE"))))))

(fn `UserConstructionScript`)