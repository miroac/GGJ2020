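; BP_Door is a double sliding door that opens on ActivateItem and closes on DeactivateItem.
; At BeginPlay it stores each leaf's world start location and a goal offset along its right vector, in opposite directions.
; Two timelines lerp the leaves between those locations, playing forward to open and stopping then reversing to close.
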(event `self.ReceiveBeginPlay`
  (bind _leftdoor (`self.LeftDoor`))
  (bind _rightdoor (`self.RightDoor`))
  (bind _returnvalue (`SceneComponent.K2_GetComponentLocation` _rightdoor))
  (set `self.RightDoorGoalLocation` (+ _returnvalue (* (`SceneComponent.GetRightVector` _rightdoor) -80.0)))
  (set `self.RightDoorStartLocation` _returnvalue)
  (set `self.LeftDoorGoalLocation` (+ (`SceneComponent.K2_GetComponentLocation` _leftdoor) (* (`SceneComponent.GetRightVector` _leftdoor) 80.0)))
  (set `self.LeftDoorStartLocation` (`SceneComponent.K2_GetComponentLocation` (`self.LeftDoor`))))

(event `self.DeactivateItem`
  (`|ExecutionSequence`
    (:`then_0`
      (bind (_direction _timeline) (`Timeline|Timeline_0` :!via `Stop` :!label _label)
        (:`Update`
          (set `self.Alpha` _timeline)
          (`SceneComponent.K2_SetWorldLocation` (`self.RightDoor`) (`KismetMathLibrary.VLerp` (`self.RightDoorStartLocation`) (`self.RightDoorGoalLocation`) (`self.Alpha`)) false false))))
    (:`then_1`
      (goto _label :!via `Reverse`))
    (:`then_2`
      (`Timeline|Timeline_1` :!via `Stop` :!label _label_2
        (:`Update`
          (`SceneComponent.K2_SetWorldLocation` (`self.LeftDoor`) (`KismetMathLibrary.VLerp` (`self.LeftDoorStartLocation`) (`self.LeftDoorGoalLocation`) (`self.Alpha`)) false false))))
    (:`then_3`
      (goto _label_2 :!via `Reverse`))))

(event `self.ActivateItem`
  (`|ExecutionSequence`
    (:`then_0`
      (goto _label))
    (:`then_1`
      (goto _label_2))))

(fn `UserConstructionScript`)