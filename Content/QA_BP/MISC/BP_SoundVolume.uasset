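; BP_SoundVolume is a one-shot trigger volume that plays a configurable sound cue when the first-person character enters it.
; It caches the QA_GM game mode on BeginPlay and, on box overlap while TriggerActive is set, calls PlayAudioSample with the game mode's audio component.
; Because playback runs on that shared component, the volume destroys itself after a zero-length delay.
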(event `self.ReceiveBeginPlay`
  (bind _asqa_gm (cast `/Game/QA_BP/GM/QA_GM` (`GameplayStatics.GetGameMode`)))
  (set `self.GameModeRef` _asqa_gm))

(event `self.Box.OnComponentBeginOverlap`
  (params (OverlappedComponent :type "PrimitiveComponent Object Reference") (OtherActor :type "Actor Object Reference") (OtherComp :type "PrimitiveComponent Object Reference") (OtherBodyIndex :type Integer) (bFromSweep :type Boolean) (SweepResult :type "HitResult Structure (by ref)"))
  (bind _gamemoderef (`self.GameModeRef`))
  (cast `/Game/FirstPersonBP/Blueprints/FirstPersonCharacter` OtherActor)
  (if (`self.TriggerActive`)
    (`/Engine/EditorBlueprintResources/StandardMacros.DoOnce` false
      (:`Completed`
        (`KismetSystemLibrary.PrintString` "Playing sound")
        (`/Game/QA_BP/GM/QA_GM.PlayAudioSample` _gamemoderef (`/Game/QA_BP/GM/QA_GM.AudioComponent` _gamemoderef) (`self.SoundCueToPlay`))
        (`KismetSystemLibrary.Delay` 0.0)
        (`self.K2_DestroyActor`)))))

(fn `UserConstructionScript`)