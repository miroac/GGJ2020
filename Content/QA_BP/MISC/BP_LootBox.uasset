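; BP_LootBox is a short-lived loot box actor that celebrates its appearance with fireworks and audio, then removes itself.
; On BeginPlay it spawns a BP_Fireworks actor just above the LootBox component, attaches it to itself and starts it after a brief delay.
; It plays the loot box sound at the player character's location, then destroys itself after a few seconds.
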(event `self.ReceiveBeginPlay`
  (bind _returnvalue_location (`KismetMathLibrary.BreakTransform` (`SceneComponent.K2_GetComponentToWorld` (`self.LootBox`))))
  (bind _returnvalue (`|SpawnActorFromClass` "/Game/QAGGJ/Effects/Fireworks/BP_Fireworks.BP_Fireworks_C" (`KismetMathLibrary.MakeTransform` (+ _returnvalue_location (0.0 0.0 5.0))) "Undefined" "OverrideRootScale" null null))
  (`self.K2_AttachToActor` _returnvalue self "None" "SnapToTarget" "KeepRelative" "KeepRelative" true)
  (`KismetSystemLibrary.Delay` 0.2)
  (`/Game/QAGGJ/Effects/Fireworks/BP_Fireworks.Start Fireworks` _returnvalue)
  (`GameplayStatics.PlaySoundAtLocation` "/Game/QAGGJ/Sound/Script/Lootbox_Audio.Lootbox_Audio" (`self.K2_GetActorLocation` (`GameplayStatics.GetPlayerCharacter` 0)) (struct) 1.0 1.0 0.0 null null null)
  (`KismetSystemLibrary.Delay` 5.0)
  (`self.K2_DestroyActor`))

(fn `UserConstructionScript`)