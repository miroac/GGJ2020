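; Interactable cookie prop with three cookie components, of which the player can eat only one.
; On the first ActivateObject, it sets an eaten flag, destroys the hit cookie by matching its component name, plays audio through the game mode and prints a debug message.
; Later activations trigger a game-mode audio call only once through DoOnce, with comments marking both voice lines as unfinished.
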(event `self.ActivateObject`
  (params (ComponentHit :type "PrimitiveComponent Object Reference"))
  (bind _gamemodereference (`self.GameModeReference`))
  (bind _gamemodereference_2 (`self.GameModeReference`))
  (if (`self.bHasACookieBeenEaten?`)
    ;[1 1 1] Put Hey youve had enough cookies here
    (`/Engine/EditorBlueprintResources/StandardMacros.DoOnce` false
      (:`Completed`
        (`/Game/QA_BP/GM/QA_GM.PlayAudioSample` _gamemodereference (`/Game/QA_BP/GM/QA_GM.AudioComponent` _gamemodereference) null)))
    (else
      (set `self.bHasACookieBeenEaten?` true)
      (switch `string` (`KismetSystemLibrary.GetObjectName` ComponentHit)
        (:`Cookie1`
          (`ActorComponent.K2_DestroyComponent` (`self.Cookie1`)))
        (:`Cookie2`
          (`ActorComponent.K2_DestroyComponent` (`self.Cookie2`)))
        (:`Cookie3`
          (`ActorComponent.K2_DestroyComponent` (`self.Cookie3`))))
      ;[1 1 1] Do we need a line here? i dont think we even have one here
      (`/Game/QA_BP/GM/QA_GM.PlayAudioSample` _gamemodereference_2 (`/Game/QA_BP/GM/QA_GM.AudioComponent` _gamemodereference_2) null)
      (`KismetSystemLibrary.PrintString` "YUM YUM"))))

(fn `UserConstructionScript`
  (`parent.UserConstructionScript`))