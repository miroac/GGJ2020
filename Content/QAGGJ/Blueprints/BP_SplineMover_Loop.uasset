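; Spline mover actor that slides a referenced ActorToMove along its spline at a set speed, in either direction.
; While its gate is open, Tick advances the distance, then wraps at the ends when Loops is set or clamps, closing the gate and disabling tick.
; BeginPlay, ActivateItem and directional events set direction and restart movement; DeactivateItem is empty.
; The construction script snaps the moved actor to the spline start.
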(event `self.ReceiveTick`
  (params (DeltaSeconds :type "Float (single-precision)"))
  (`/Engine/EditorBlueprintResources/StandardMacros.Gate` true :!label _label
    (:`Exit`
      (set `self.DistanceAlongSpline` (+ (`self.DistanceAlongSpline`) (* (`self.Direction`) (* (`self.MovementSpeed`) (`GameplayStatics.GetWorldDeltaSeconds`)))))
      (if (`self.Loops`)
        (if (>= (`self.DistanceAlongSpline`) (`SplineComponent.GetSplineLength` (`self.Spline`)))
          (set `self.DistanceAlongSpline` 0.0)
          (elif (< (`self.DistanceAlongSpline`) 0.0)
            (set `self.DistanceAlongSpline` (`SplineComponent.GetSplineLength` (`self.Spline`)))))
        (`self.K2_SetActorLocation` (`self.ActorToMove`) (`SplineComponent.GetLocationAtDistanceAlongSpline` (`self.Spline`) (`self.DistanceAlongSpline`) "World") false false)
        (elif (>= (`self.DistanceAlongSpline`) (`SplineComponent.GetSplineLength` (`self.Spline`)))
          (set `self.DistanceAlongSpline` (`SplineComponent.GetSplineLength` (`self.Spline`)))
          (`|ExecutionSequence`
            (:`then_0`
              (`self.CloseGate`))
            (:`then_1`
              (`self.K2_SetActorLocation` (`self.ActorToMove`) (`SplineComponent.GetLocationAtDistanceAlongSpline` (`self.Spline`) (`self.DistanceAlongSpline`) "World") false false :!label _label_2)))
          (elif (< (`self.DistanceAlongSpline`) 0.0)
            (`|ExecutionSequence`
              (:`then_0`
                (`self.CloseGate`))
              (:`then_1`
                (set `self.DistanceAlongSpline` 0.0)
                (goto _label_2)))
            (else
              (goto _label_2))))))))

(event `MoveAtoB`
  (set `self.Direction` 1 :!label _label_3)
  (if (== (`self.DistanceAlongSpline`) (`SplineComponent.GetSplineLength` (`self.Spline`)))
    (set `self.DistanceAlongSpline` 0.0))
  (`self.SetActorTickEnabled` true :!label _label_4)
  (goto _label :!via `Open`))

(event `self.ReceiveBeginPlay`
  (`parent.ReceiveBeginPlay`)
  (if (`self.bMoveAToB?`) :!label _label_5
    (goto _label_3)
    (else
      (set `self.Direction` -1 :!label _label_6)
      (if (== (`self.DistanceAlongSpline`) 0.0)
        (set `self.DistanceAlongSpline` (`SplineComponent.GetSplineLength` (`self.Spline`)))
        (goto _label_4)
        (else
          (goto _label_4))))))

(event `self.ActivateItem`
  (`self.SetActorTickEnabled` true)
  (goto _label_5))

(event `MoveBtoA`
  (goto _label_6))

(event `CloseGate`
  (`self.SetActorTickEnabled` false)
  (goto _label :!via `Close`))

(event `self.DeactivateItem`)

(fn `UserConstructionScript`
  (`self.K2_SetActorLocation` (`self.ActorToMove`) (`SplineComponent.GetLocationAtTime` (`self.Spline`) 0.0 "World" false) false false))