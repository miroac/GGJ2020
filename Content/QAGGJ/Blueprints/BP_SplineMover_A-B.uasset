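; Spline mover that slides a referenced actor back and forth between the two ends of a spline at a set speed.
; BeginPlay and ActivateItem start travel in the MoveAToB direction, while MoveAtoB and MoveBtoA force a direction.
; A gated Tick advances and clamps the spline distance, switching itself off at either end or on DeactivateItem.
; The construction script snaps the actor to the spline start.
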(event `self.ReceiveTick`
  (params (DeltaSeconds :type "Float (single-precision)"))
  (`/Engine/EditorBlueprintResources/StandardMacros.Gate` true :!label _label
    (:`Exit`
      (bind _output_get (set `self.DistanceAlongSpline` (+ (`self.DistanceAlongSpline`) (* (`self.Direction`) (* (`self.MovementSpeed`) (`GameplayStatics.GetWorldDeltaSeconds`))))))
      (if (>= _output_get (`SplineComponent.GetSplineLength` (`self.Spline`)))
        (set `self.DistanceAlongSpline` (`SplineComponent.GetSplineLength` (`self.Spline`)))
        (`|ExecutionSequence`
          (:`then_0`
            (`self.CloseGate`))
          (:`then_1`
            (`self.K2_SetActorLocation` (`self.ActorToMove`) (`SplineComponent.GetLocationAtDistanceAlongSpline` (`self.Spline`) (`self.DistanceAlongSpline`) "World") false false :!label _label_2)))
        (elif (< (`self.DistanceAlongSpline`) 0.0)
          (`|ExecutionSequence`
            (:`then_0`
              (`self.CloseGate`))
            (:`then_1`
              (set `self.DistanceAlongSpline` 0.0)
              (goto _label_2)))
          (else
            (goto _label_2)))))))

(event `self.ReceiveBeginPlay`
  (if (`self.bMoveAToB?`) :!label _label_3
    (set `self.Direction` 1 :!label _label_4)
    (else
      (set `self.Direction` -1 :!label _label_5)))
  (`self.SetActorTickEnabled` true)
  (goto _label :!via `Open`))

(event `MoveAtoB`
  (goto _label_4))

(event `self.ActivateItem`
  (goto _label_3))

(event `MoveBtoA`
  (goto _label_5))

(event `CloseGate`
  (`self.SetActorTickEnabled` false :!label _label_6)
  (goto _label :!via `Close`))

(event `self.DeactivateItem`
  (goto _label_6))

(fn `UserConstructionScript`
  (`self.K2_SetActorLocation` (`self.ActorToMove`) (`SplineComponent.GetLocationAtTime` (`self.Spline`) 0.0 "World" false) false false))