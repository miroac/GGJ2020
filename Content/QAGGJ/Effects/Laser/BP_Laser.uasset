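; BP_Laser is a laser beam that a gun can grab and attach to a new node or release, collapsing it.
; While active, Tick stretches and aims the mesh at EndPoint and fits the hum's capsule attenuation to the beam.
; While grabbed, it follows the gun's socket and sphere-traces along itself, feeding obstacle proximity to its dynamic material.
; TriggerPower and KillPower run timelines that animate the material's transition, powering down five times faster.
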(event `self.ReceiveBeginPlay`
  (bind _outactors (`GameplayStatics.GetAllActorsOfClass` "/Game/QA_BP/Nodes/BP_BaseNode.BP_BaseNode_C"))
  (bind _output_get (set `self.ActorsToIgnore` _outactors))
  (`KismetArrayLibrary.Array_Add` _output_get (`GameplayStatics.GetPlayerPawn` 0))
  (`TimelineComponent.SetPlaybackPosition` (`self.PoweringForward`) 1.0 false true)
  (`MaterialInstanceDynamic.SetScalarParameterValue` (`self.SideInstance`) "TransitionAmount" 0.0)
  (set `self.PowerValue` 0.0)
  (if (`self.StartActive`)
    (`self.ActivateLaser`)
    (else
      (`self.DeactivateLaser`))))

(event `self.ReceiveTick`
  (params (DeltaSeconds :type "Float (single-precision)"))
  (`|ExecutionSequence`
    (:`then_0`
      (`self.UpdateLaserGraphics`)
      (if (`self.IsGrabbed`)
        (`MaterialInstanceDynamic.SetScalarParameterValue` (`self.SideInstance`) "GrabbedSwitch" 1.0)
        (`MaterialInstanceDynamic.SetScalarParameterValue` (`self.SideInstance`) "DistanceChecker" (`self.CloseCallChecker` (`self.DistanceCheckRadius`)))
        (else
          (`MaterialInstanceDynamic.SetScalarParameterValue` (`self.SideInstance`) "DistanceChecker" 0.0)
          (`MaterialInstanceDynamic.SetScalarParameterValue` (`self.SideInstance`) "GrabbedSwitch" 0.0))))))

(event `PowerSwitch`
  (if (`self.IsPowered`)
    (`TimelineComponent.SetPlayRate` (`self.PoweringForward`) (/ 1.0 (`self.Speed`)))
    (`TimelineComponent.SetPlaybackPosition` (`self.PoweringForward`) (`self.PowerValue`) false true)
    (bind (_direction _powervalue) (`Timeline|PoweringForward`)
      (:`Update`
        (bind _output_get (set `self.PowerValue` _powervalue))
        (`KismetSystemLibrary.PrintString` (`KismetStringLibrary.Conv_DoubleToString` _output_get))))
    (else
      (`TimelineComponent.SetPlayRate` (`self.PoweringReverse`) (* (/ 1.0 (`self.Speed`)) 5.0))
      (`TimelineComponent.SetPlaybackPosition` (`self.PoweringForward`) (`KismetMathLibrary.Lerp` 1.0 0.0 (`self.PowerValue`)) false true)
      (bind (_direction_2 _powervalue_2) (`Timeline|PoweringReverse`)
        (:`Update`
          (set `self.PowerValue` _powervalue_2)))))
  (`MaterialInstanceDynamic.SetScalarParameterValue` (`self.SideInstance`) "TransitionAmount" (`self.PowerValue`)))

(fn `ActivateLaser`
  (`SceneComponent.SetVisibility` (`self.SM_Laser`) true false)
  (`self.SetActorTickEnabled` true))

(fn `CloseCallChecker`
  (params (Radius :type "Float (double-precision)" :default 1000.0))
  (returns (DistanceToCentre :type "Float (double-precision)"))
  (locals (HitTime :type "Float (double-precision)" :default 0.0) (HitDirection :type "Vector Structure" :default (0.0 0.0 0.0)))
  (bind _returnvalue (`self.K2_GetActorLocation`))
  (bind _endpoint (`self.EndPoint`))
  (set `local.HitDirection` (`KismetMathLibrary.Normal` (- (`self.K2_GetActorLocation`) (`self.EndPoint`))))
  (`SplineComponent.SetSplinePoints` (`self.RadiusChecker`) (`|MakeArray` _returnvalue _endpoint) "World" true)
  (bind _outhit (`KismetSystemLibrary.SphereTraceSingle` _returnvalue _endpoint (`local.Radius`) "TraceTypeQuery1" false (`self.ActorsToIgnore`) (cast `EDrawDebugTrace` (`KismetMathLibrary.Conv_BoolToByte` (`self.DebugEnabled`)))))
  (bind (_bblockinghit _binitialoverlap _time _distance _location _impactpoint _normal _impactnormal _physmat _hitactor) (`GameplayStatics.BreakHitResult` _outhit))
  (bind _returnvalue_2 (`KismetSystemLibrary.GetObjectName` _hitactor))
  (if (or (`KismetStringLibrary.Contains` _returnvalue_2 "modelcomponent") (`KismetStringLibrary.Contains` _returnvalue_2 "reroute"))
    _
    (elif _bblockinghit
      (return (`KismetMathLibrary.Lerp` 1.0 0.0 (/ (`KismetMathLibrary.FClamp` (`KismetMathLibrary.VSize` (- (+ (`SplineComponent.GetLocationAtTime` (`self.RadiusChecker`) _time "World" false) (* (`local.HitDirection`) (* -1 (`local.Radius`)))) _impactpoint)) 0.0 (`local.Radius`)) (`local.Radius`))))
      (else
        (return 0.0)))))

(fn `DeactivateLaser`
  (`SceneComponent.SetVisibility` (`self.SM_Laser`) false false)
  (`self.SetActorTickEnabled` false))

(fn `GetLengthOfLaser`
  (returns (LengthOfLaser :type "Float (double-precision)"))
  (return (`KismetMathLibrary.VSize` (- (`self.K2_GetActorLocation`) (`self.EndPoint`)))))

(fn `KillPower`
  (set `self.IsPowered` false)
  (`self.PowerSwitch`))

(fn `LaserBroken`
  (set `self.IsGrabbed` false)
  (set `self.EndPoint` (`self.K2_GetActorLocation`)))

(fn `LaserGrabbed`
  (params (Gun :type "SkeletalMeshComponent Object Reference"))
  (set `self.GunComponent` Gun)
  (set `self.IsGrabbed` true))

(fn `LaserReleased`
  (params (IsLaserAtNewNode :type Boolean) (NewEndLocation :type "Vector Structure"))
  (if IsLaserAtNewNode
    (set `self.EndPoint` NewEndLocation)
    (set `self.IsGrabbed` false)
    (else
      (set `self.EndPoint` (`self.K2_GetActorLocation`))
      (set `self.IsGrabbed` false))))

(fn `TriggerPower`
  (params (Speed :type "Float (double-precision)"))
  (set `self.Speed` Speed)
  (set `self.IsPowered` true)
  (`self.PowerSwitch`))

(fn `UpdateLaserGraphics`
  (bind _returnvalue (`KismetMathLibrary.FindLookAtRotation` (`self.K2_GetActorLocation`) (`self.EndPoint`)))
  (if (`self.IsGrabbed`)
    (bind _guncomponent (`self.GunComponent`)
      (:`then`
        (set `self.EndPoint` (`SceneComponent.GetSocketLocation` _guncomponent "LaserSocket")))
      (:`else`
        _)))
  (`SceneComponent.SetRelativeScale3D` (`self.SM_Laser`) (`KismetMathLibrary.MakeVector` (/ (`KismetMathLibrary.VSize` (- (`self.K2_GetActorLocation`) (`self.EndPoint`))) 20.0) 0.2 0.2))
  (`SceneComponent.K2_SetRelativeRotation` (`self.SM_Laser`) _returnvalue false false)
  (`SceneComponent.K2_SetRelativeRotation` (`self.HummerLoc`) _returnvalue false false)
  (`SceneComponent.K2_SetWorldLocation` (`self.HummerLoc`) (/ (+ (`self.K2_GetActorLocation`) (`self.EndPoint`)) 2.0) false false)
  (if (== (`self.K2_GetActorLocation`) (`self.EndPoint`))
    (set `self.CapsuleHeight` 0.0)
    (set `self.CapsuleRadius` 0.0)
    (else
      (set `self.CapsuleHeight` (/ (`KismetMathLibrary.VSize` (- (`self.K2_GetActorLocation`) (`self.EndPoint`))) 2.0))
      (set `self.CapsuleRadius` 100.0)))
  (`AudioComponent.AdjustAttenuation` (`self.Electrical-hum-loop`) (make `SoundAttenuationSettings` :`AttenuationShape` "Capsule" :`AttenuationShapeExtents` (`KismetMathLibrary.MakeVector` (`self.CapsuleHeight`)) :`FalloffDistance` (`self.CapsuleRadius`))))

(fn `UserConstructionScript`
  (set `AudioComponent.AttenuationOverrides` (make `SoundAttenuationSettings` :`AttenuationShape` "Capsule" :`AttenuationShapeExtents` (0.0 0.0 0.0) :`FalloffDistance` 0.0) (`self.Electrical-hum-loop`))
  (bind _returnvalue (`KismetMaterialLibrary.CreateDynamicMaterialInstance` "/Game/QAGGJ/Effects/Laser/M_LaserSide.M_LaserSide" "LaserSide"))
  (bind _output_get (set `self.SideInstance` _returnvalue))
  (`PrimitiveComponent.SetMaterial` (`self.SM_Laser`) 0 _output_get)
  (`self.UpdateLaserGraphics`)
  (`SplineComponent.SetSplinePoints` (`self.RadiusChecker`) (`|MakeArray` (`self.K2_GetActorLocation`) (`self.EndPoint`)) "World" true))