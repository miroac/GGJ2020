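; Fireworks spawner actor that repeatedly launches Niagara fireworks at random points within a Range box oriented to and centred on the actor.
; StartFireworks and StopFireworks toggle Tick and a Gate that feeds a DoOnce, re-armed after a random delay to pace the bursts.
; Each burst spawns NS_Fireworks with auto-destroy off and sets its colour parameter from a random-hue colour scaled by an emissive multiplier.
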(event `self.ReceiveTick`
  (params (DeltaSeconds :type "Float (single-precision)"))
  (bind _color (`self.Color`))
  (bind _returnvalue (/ (.x (`self.Range`)) 2.0))
  (bind _returnvalue_2 (/ (.y (`self.Range`)) 2.0))
  (bind _returnvalue_3 (/ (.z (`self.Range`)) 2.0))
  (`/Engine/EditorBlueprintResources/StandardMacros.Gate` true :!label _label
    (:`Exit`
      (`|ExecutionSequence`
        (:`then_0`
          (`/Engine/EditorBlueprintResources/StandardMacros.DoOnce` false :!label _label_2
            (:`Completed`
              (bind _returnvalue_4 (`NiagaraFunctionLibrary.SpawnSystemAtLocation` "/Game/QAGGJ/Effects/Fireworks/NS_Fireworks.NS_Fireworks" (+ (* (`self.GetActorForwardVector`) (`KismetMathLibrary.RandomFloatInRange` (* -1.0 _returnvalue) _returnvalue)) (* (`self.GetActorRightVector`) (`KismetMathLibrary.RandomFloatInRange` (* -1.0 _returnvalue_2) _returnvalue_2)) (* (`self.GetActorUpVector`) (`KismetMathLibrary.RandomFloatInRange` (* -1.0 _returnvalue_3) _returnvalue_3)) (`self.K2_GetActorLocation`)) (struct) (1.0 1.0 1.0) false))
              (`KismetMathLibrary.LinearColor_SetRandomHue` _color)
              (`FXSystemComponent.SetColorParameter` _returnvalue_4 "User.FireworksColour" (* _color (`self.EmissiveMulti`))))))
        (:`then_1`
          (`KismetSystemLibrary.Delay` (`KismetMathLibrary.RandomFloatInRange` (`self.DelayMax`) (`self.DelayMin`)))
          (goto _label_2 :!via `Reset`))))))

(event `Start Fireworks`
  (`self.SetActorTickEnabled` true)
  (goto _label :!via `Open`))

(event `StopFireworks`
  (`self.SetActorTickEnabled` false)
  (goto _label :!via `Close`))

(fn `UserConstructionScript`)