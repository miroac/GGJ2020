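; BP_AutoDoor is a child door Blueprint that configures a single swinging door for the automatic door system in the Blocking Starter Pack.
; Its construction script yaws the RightOpenPosition component by the negated RightDoorOpening angle.
; It also rebuilds DoorParts as one entry, with closed and open transforms sharing an offset and differing only in that yaw.
; It then runs the parent construction script, after that data is set.
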(fn `UserConstructionScript`
  (`SceneComponent.K2_SetRelativeRotation` (`self.RightOpenPosition`) (`KismetMathLibrary.MakeRotator` 0.0 0.0 (* (`self.RightDoorOpening`) -1.0)) false false)
  (set `self.DoorParts` (`|MakeArray` (make `/Game/BlockingStarterPack/Blueprints/AutomaticDoor/DoorParts_Struct` (`self.DoorMesh`) (`|MakeArray`) (`KismetMathLibrary.MakeTransform` (50.0 0.0 0.0)) (`KismetMathLibrary.MakeTransform` (50.0 0.0 0.0) (`KismetMathLibrary.MakeRotator` 0.0 0.0 (* (`self.RightDoorOpening`) -1.0))))))
  (`parent.UserConstructionScript`))